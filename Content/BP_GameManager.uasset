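; Game manager that owns the UI widgets and handles the flow between main menu, levels and pause.
; Init creates and caches the HUD, menu, instruction, controller, win/lose, pause and settings widgets.
; Level and menu loads run asynchronously, swapping widgets, input mode and cursor, while driving the shift timer, score saving, music and character reset.
; PauseGame toggles pause, the pause widget and the cursor.
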(event Custom|LoadMenu
  (bind _customcontroller (CallFunction|GetGameController))
  (bind _menu (Variables|Default|GetMenu))
  ;[0.15 0.15 0.15 0.5] Loads menu
  (Class|ScoreManager|SaveScore (Subsystems|GetScoreManager))
  (Default|UpdateHighscoreUI _menu)
  (UserInterface|Viewport|AddtoViewport _menu 0)
  (|LoadLevelAsync "/Game/Levels/Menu.Menu"
    (:then
      (Widget|RemovefromParent (Variables|Default|GetHud)))
    (:OnLevelLoaded
      (Variables|/Script/Engine.PlayerController|SetbShowMouseCursor _customcontroller true)
      (Input|SetInputModeUIOnly _customcontroller 0 "DoNotLock" false)
      (bind _returnvalue (Class|FMODBlueprintStatics|PlayEvent2D "/Game/FMOD/Events/Music/Mu_MainMenu.Mu_MainMenu"))
      (Variables|Default|SetMusicInstance _returnvalue)
      (Default|ResetCharacter (CallFunction|GetPlayerCharacter)))))

(event Custom|Load%20Level
  (bind _customcontroller (CallFunction|GetGameController))
  (bind _musicinstance (Variables|Default|GetMusicInstance))
  ;[0.15 0.15 0.15 0.5] Loads level from level button
  (Class|ShiftManager|SetShiftTime (Subsystems|GetShiftManager) (Variables|Default|GetLevelTime))
  (bind _returnvalue (Class|FMODBlueprintStatics|EventInstanceIsValid _musicinstance))
  (if _returnvalue
    (Class|FMODBlueprintStatics|EventInstanceStop _musicinstance false))
  (Class|ShiftManager|StartTimer (Subsystems|GetShiftManager))
  (UserInterface|Viewport|AddtoViewport (Variables|Default|GetHud) 0)
  (|LoadLevelAsync (Variables|Default|GetLevel)
    (:then
      (Widget|RemovefromParent (Variables|Default|GetMenu))
      (Widget|RemovefromParent (Variables|Default|GetInstructionWidget)))
    (:OnLevelLoaded
      (Variables|/Script/Engine.PlayerController|SetbShowMouseCursor _customcontroller false)
      (Input|SetInputModeGameOnly _customcontroller false))))

(event EventPauseGame
  (Game|SetGamePaused (Class|KismetMathLibrary|XORBoolean (Game|IsGamePaused) true))
  (if (Game|IsGamePaused)
    (UserInterface|Viewport|AddtoViewport (Variables|Default|GetPauseWidget) 0)
    (else
      (Widget|RemovefromParent (Variables|Default|GetPauseWidget))))
  (Variables|/Script/Engine.PlayerController|SetbShowMouseCursor (CallFunction|GetGameController) (Game|IsGamePaused)))

(event EventInit
  ;[0.15 0.15 0.15 0.5] Loads all necessary widgets
  (Utilities|FlowControl|Sequence
    (:then_0
      (bind _returnvalue (UserInterface|CreateWidget "/Game/Widgets/WBP_HUD.WBP_HUD_C"))
      (Variables|Default|SetHud _returnvalue)
      (bind _returnvalue_2 (UserInterface|CreateWidget "/Game/Widgets/WBP_Menu.WBP_Menu_C"))
      (Variables|Default|SetMenu _returnvalue_2)
      (bind _returnvalue_3 (UserInterface|CreateWidget "/Game/Widgets/WBP_InstructionFlowChart.WBP_InstructionFlowChart_C"))
      (Variables|Default|SetInstructionWidget _returnvalue_3)
      (bind _returnvalue_4 (UserInterface|CreateWidget "/Game/Widgets/WBP_ControllerMap.WBP_ControllerMap_C"))
      (Variables|Default|SetControllerWidget _returnvalue_4))
    (:then_1
      (bind _returnvalue_5 (UserInterface|CreateWidget "/Game/Widgets/WBP_WinOrLoseScreen.WBP_WinOrLoseScreen_C"))
      (Variables|Default|SetWinOrLoseWidget _returnvalue_5)
      (bind _returnvalue_6 (UserInterface|CreateWidget "/Game/Widgets/WBP_Pause.WBP_Pause_C"))
      (Variables|Default|SetPauseWidget _returnvalue_6)
      (bind _returnvalue_7 (UserInterface|CreateWidget "/Game/Widgets/WBP_Settings.WBP_Settings_C"))
      (Variables|Default|SetSettingsWidget _returnvalue_7))))