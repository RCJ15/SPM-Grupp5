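; Item component that can turn its owning item into a bomb and can break other actors.
; BecomeABomb acts only while the owner is inspected: it removes the FragileComponent, swaps in the bomb mesh and material, then calls SetValues on BP_Item.
; An author note flags this conversion as not working.
; BreakCaller calls Break on any passed actor implementing CanBeBroken; no detonation logic or triggers are defined here.
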(event Custom|BecomeABomb
  (bind _owner (Variables|Default|GetOwner))
  (bind _basemesh (Variables|/Script/SpmG5.Item|GetBaseMesh _owner))
  (if (Class|Item|GetIsInspected (Variables|Default|GetOwner))
    ;[1 0 0.02028 0.5] Kanske ta bort mer typ?
    (Components|DestroyComponent (Actor|GetComponentbyClass _owner "/Script/SpmG5.FragileComponent"))
    (Components|StaticMesh|SetStaticMesh _basemesh "/Game/Meshes/SM_Bomb.SM_Bomb")
    (Rendering|Material|SetMaterial _basemesh 0 "/Game/Materials/3D/Bomb/M_Bomb.M_Bomb")
    (Default|SetValues (.AsBP%20Item (Utilities|Casting|CastToBP_Item (Variables|Default|GetOwner))))))

(event EventBeginPlay)

(event EventTick
  (params (DeltaSeconds :type Float%20%28single-precision%29)))

(event EventBreakCaller
  (params (Actor :type Actor%20Object%20Reference))
  (bind _ascan_be_broken (Utilities|Casting|CastToCanBeBroken Actor))
  (Class|CanbeBroken|Break _ascan_be_broken))