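; BP_SpinningCross is a level component actor that spins continuously in 90-degree yaw steps.
; Shortly after BeginPlay it stores the static mesh's world yaw, then sets a target a quarter turn further.
; A timeline lerps the actor's relative yaw to that target with sweep enabled, and on finishing stores it and starts the next step, looping indefinitely.
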(event Custom|SetRotation
  (bind _spin (Timeline|Timeline PlayFromStart)
    (:Update
      (Transformation|SetActorRelativeRotation (Math|Rotator|MakeRotator 0.0 0.0 (Math|Float|Lerp (Variables|Default|GetRotation) (Variables|Default|GetNewRotation) _spin)) true))
    (:Finished
      (Variables|Default|SetRotation (Variables|Default|GetNewRotation))
      (CallFunction|GetNewRotation))))

(event Custom|GetNewRotation
  (Variables|Default|SetNewRotation (+ (Variables|Default|GetRotation) 9e+01))
  (CallFunction|SetRotation))

(event EventBeginPlay
  (Utilities|FlowControl|Delay 0.2)
  (Variables|Default|SetRotation (.yaw (Transformation|GetWorldRotation (Variables|Default|GetStaticMesh))))
  (CallFunction|GetNewRotation))

(fn ConstructionScript)