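; BP_SpinningCentre is a level component actor that rotates around its vertical axis in repeating quarter-turn steps.
; On BeginPlay it stores the static mesh's world yaw, then sets a target 90 degrees further on.
; After a configurable delay, a timeline interpolates the actor's relative yaw to that target, then stores it and starts the next step, looping indefinitely.
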(event Custom|SetRotation
  (Utilities|FlowControl|Delay (Variables|Default|GetDelay))
  (bind _spin (Timeline|Timeline PlayFromStart)
    (:Update
      (Transformation|SetActorRelativeRotation (Math|Rotator|MakeRotator 0.0 0.0 (Math|Float|Lerp (Variables|Default|GetRotation) (Variables|Default|GetNewRotation) _spin))))
    (:Finished
      (Variables|Default|SetRotation (Variables|Default|GetNewRotation))
      (CallFunction|GetNewRotation))))

(event Custom|GetNewRotation
  (Variables|Default|SetNewRotation (+ (Variables|Default|GetRotation) 9e+01))
  (CallFunction|SetRotation))

(event EventBeginPlay
  (Variables|Default|SetRotation (.yaw (Transformation|GetWorldRotation (Variables|Default|GetStaticMesh))))
  (CallFunction|GetNewRotation))

(fn ConstructionScript)