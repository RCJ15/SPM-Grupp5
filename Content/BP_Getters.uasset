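; BP_Getters is a set of shared helper functions that return the game's core custom objects, already cast to their Blueprint types.
; GetGameManager casts the game instance to BP_GameManager, and GetGameController casts player controller 0 to BP_CustomController.
; GetPlayerCharacter builds on GetGameController, passing its controller ID as the player index to fetch the pawn as BP_CustomCharacter.
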(fn GetGameManager
  (bind _asbp_game_manager (Utilities|Casting|CastToBP_GameManager (Game|GetGameInstance (LocalVariables|Get__WorldContext))))
  (return _asbp_game_manager))

(fn GetGameController
  (bind _asbp_custom_controller (Utilities|Casting|CastToBP_CustomController (Game|GetPlayerController 0)))
  (return _asbp_custom_controller))

(fn GetPlayerCharacter
  (bind _customcontroller (CallFunction|GetGameController (LocalVariables|Get__WorldContext)))
  (bind _asbp_custom_character (Utilities|Casting|CastToBP_CustomCharacter (Game|Player|GetPlayerPawn 0 (Class|GameplayStatics|GetPlayerControllerID _customcontroller))))
  (return _asbp_custom_character))