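; BP_DoorTrigger is a level component Blueprint that triggers interactions on an assigned set of doors at random intervals.
; On BeginPlay it waits a random time between DelayMin and DelayMax, then calls DoorInteraction on each entry in Doors.
; The loop body calls StartDelay again for each door, so the cycle repeats indefinitely as long as the array has entries.
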(event Custom|DoorInteract
  (for _array_element (Variables|Default|GetDoors)
    (Default|DoorInteraction _array_element)
    (CallFunction|StartDelay)))

(event Custom|StartDelay
  (Utilities|FlowControl|Delay (Math|Random|RandomFloatinRange (Variables|Default|GetDelayMin) (Variables|Default|GetDelayMax)))
  (CallFunction|DoorInteract))

(event EventBeginPlay
  (CallFunction|StartDelay))

(fn ConstructionScript)