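; BP_OneSidedGate is a gate that swings open while SpmG5Character actors overlap it.
; Overlap events maintain a StandingPeople count, playing the RotationProgress timeline on entry and reversing it once the count drops to zero.
; The timeline's Degrees track drives the Gate's relative yaw, and on entry the timeline time is set from Degrees / 90 to match the current angle.
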(event Collision|EventActorEndOverlap
  (params (OtherActor :type Actor%20Object%20Reference))
  (Utilities|Casting|CastToSpmG5Character OtherActor)
  (bind _output_get (Variables|Default|SetStandingPeople (- (Variables|Default|GetStandingPeople) 1)))
  (if (<= _output_get 0)
    (Utilities|FlowControl|Sequence
      (:then_0
        (bind _degrees (Timeline|RotationProgress SetNewTime)
          (:Update
            (bind _output_get_2 (Variables|Default|SetDegrees _degrees))
            (Transformation|SetRelativeRotation (Variables|Default|GetGate) (Math|Rotator|MakeRotator 0.0 0.0 _output_get_2) false false))))
      (:then_1
        (Timeline|RotationProgress Reverse)))))

(event Collision|EventActorBeginOverlap
  (params (OtherActor :type Actor%20Object%20Reference))
  (Utilities|Casting|CastToSpmG5Character OtherActor)
  (Variables|Default|SetStandingPeople (+ (Variables|Default|GetStandingPeople) 1))
  (Utilities|FlowControl|Sequence
    (:then_0
      (bind _degrees (Timeline|RotationProgress SetNewTime)
        (:Update
          (bind _output_get (Variables|Default|SetDegrees _degrees))
          (Transformation|SetRelativeRotation (Variables|Default|GetGate) (Math|Rotator|MakeRotator 0.0 0.0 _output_get) false false))))
    (:then_1
      (Timeline|RotationProgress Play))))

(fn ConstructionScript)