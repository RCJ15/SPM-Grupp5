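; Tutorial controller that runs four box-sorting tests in sequence, then loads the menu.
; Each test sets a target score and box count, then spawns circle and triangle items varying in address-decal visibility or suspicious flag.
; Score-change events tally results; an exact score match on the last box advances, otherwise the test repeats.
; ChangeTest shows the matching tutorial widget page, and the second test spawns another wave after a delay.
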(event Custom|CheckBox
  (bind _returnvalue (Class|ScoreManager|GetAddedScore (Subsystems|GetScoreManager)))
  (Variables|Default|SetTotalScore (+ (Variables|Default|GetTotalScore) _returnvalue))
  (if (== (Variables|Default|GetSortedBoxes) (Variables|Default|GetBoxesToSort))
    (if (== (Variables|Default|GetScoreToPass) (Variables|Default|GetTotalScore))
      (Variables|Default|SetSortedBoxes 1)
      (Variables|Default|SetTotalScore 0)
      (Variables|Default|SetPassedTests (+ (Variables|Default|GetPassedTests) 1))
      (UserInterface|Viewport|AddtoViewport (Variables|Default|GetTutorialWidget) 0)
      (else
        (Variables|Default|SetSortedBoxes 1)
        (Variables|Default|SetTotalScore 0)))
    (CallFunction|ChangeTest)
    (Utilities|FlowControl|Delay 3.0)
    (if (Variables|Default|GetIsSecondTest)
      (CallFunction|SecondTest)
      (Variables|Default|SetIsSecondTest false))
    (else
      (Variables|Default|SetSortedBoxes (+ (Variables|Default|GetSortedBoxes) 1)))))

(event EventBeginPlay
  (bind _tutorialwidget (Variables|Default|GetTutorialWidget))
  (Utilities|FlowControl|Delay 0.2)
  (EventDispatchers|BindEventtoOnScoreChanged (Subsystems|GetScoreManager) (delegate Custom|CheckBox))
  (UserInterface|Viewport|AddtoViewport _tutorialwidget 0)
  (Input|SetInputModeUIOnly (.CustomController1 (CallFunction|GetGameController)) _tutorialwidget "DoNotLock" false)
  (CallFunction|ChangeTest))

(event EventTick
  (params (DeltaSeconds :type Float%20%28single-precision%29)))

(fn ChangeTest
  (if (<= (Variables|Default|GetPassedTests) 0)
    (CallFunction|FirstTest)
    (Default|ShowTutorialbyIndex (Variables|Default|GetTutorialWidget) (Variables|Default|GetPassedTests))
    (Input|SetInputModeUIOnly (.CustomController1 (CallFunction|GetGameController)) (Variables|Default|GetTutorialWidget) "DoNotLock" false :!label _label)
    (Class|Widget|SetUserFocus (Variables|Default|GetTutorialWidget) (.CustomController1 (CallFunction|GetGameController)))
    (elif (<= (Variables|Default|GetPassedTests) 1)
      (CallFunction|SecondTest)
      (Default|ShowTutorialbyIndex (Variables|Default|GetTutorialWidget) (Variables|Default|GetPassedTests))
      (goto _label)
      (elif (<= (Variables|Default|GetPassedTests) 2)
        (CallFunction|ThirdTest)
        (Default|ShowTutorialbyIndex (Variables|Default|GetTutorialWidget) (Variables|Default|GetPassedTests))
        (goto _label)
        (elif (<= (Variables|Default|GetPassedTests) 3)
          (CallFunction|FourthTest)
          (Default|ShowTutorialbyIndex (Variables|Default|GetTutorialWidget) (Variables|Default|GetPassedTests))
          (goto _label)
          (else
            (Default|LoadMenu (CallFunction|GetGameManager))))))))

(fn FirstTest
  (Variables|Default|SetScoreToPass 10)
  (Variables|Default|SetBoxesToSort 2)
  (for (_array_element _array_index) (Variables|Default|GetSpawnManeger)
    (if (== _array_index 0)
      (bind _returnvalue (Class|BoxSpawner|SpawnItem _array_element false false false false "CIRCLE"))
      (Rendering|SetVisibility (Actor|GetComponentbyClass _returnvalue "/Script/Engine.DecalComponent") (Variables|Default|GetHas%20Adress) false)
      (else
        (bind _returnvalue_2 (Class|BoxSpawner|SpawnItem _array_element false false false false "TRIANGLE"))
        (Rendering|SetVisibility (Actor|GetComponentbyClass _returnvalue_2 "/Script/Engine.DecalComponent") (Variables|Default|GetHas%20Adress) false)))))

(fn SecondTest
  (Variables|Default|SetIsSecondTest true)
  (Development|PrintString "2!")
  (Variables|Default|SetScoreToPass 40)
  (Variables|Default|SetBoxesToSort 4)
  (Variables|Default|SetHas%20Adress false)
  (for (_array_element _array_index) (Variables|Default|GetSpawnManeger)
    (if (== _array_index 0)
      (bind _returnvalue (Class|BoxSpawner|SpawnItem _array_element false false false false "CIRCLE"))
      (Rendering|SetVisibility (Actor|GetComponentbyClass _returnvalue "/Script/Engine.DecalComponent") (Variables|Default|GetHas%20Adress) false)
      (else
        (bind _returnvalue_2 (Class|BoxSpawner|SpawnItem _array_element false false false false "TRIANGLE"))
        (Rendering|SetVisibility (Actor|GetComponentbyClass _returnvalue_2 "/Script/Engine.DecalComponent") (Variables|Default|GetHas%20Adress) false)))))

(fn ThirdTest
  (Variables|Default|SetScoreToPass 30)
  (Variables|Default|SetBoxesToSort 2)
  (for (_array_element _array_index) (Variables|Default|GetSpawnManeger)
    (if (== _array_index 0)
      (Class|BoxSpawner|SpawnItem _array_element false false false true "CIRCLE")
      (else
        (Class|BoxSpawner|SpawnItem _array_element false false false true "TRIANGLE")))))

(fn FourthTest
  (Variables|Default|SetHas%20Adress true)
  (Variables|Default|SetScoreToPass 10)
  (Variables|Default|SetBoxesToSort 2)
  (for (_array_element _array_index) (Variables|Default|GetSpawnManeger)
    (if (== _array_index 0)
      (bind _returnvalue (Class|BoxSpawner|SpawnItem _array_element false false false false "TRIANGLE"))
      (Rendering|SetVisibility (Actor|GetComponentbyClass _returnvalue "/Script/Engine.DecalComponent") (Variables|Default|GetHas%20Adress) false)
      (else
        (bind _returnvalue_2 (Class|BoxSpawner|SpawnItem _array_element false false false false "CIRCLE"))
        (Rendering|SetVisibility (Actor|GetComponentbyClass _returnvalue_2 "/Script/Engine.DecalComponent") (Variables|Default|GetHas%20Adress) false)))))