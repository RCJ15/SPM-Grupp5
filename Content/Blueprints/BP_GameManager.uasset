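; Central game manager for a two-player box-shift game, handling widgets, level flow, pausing and save data.
; Init creates the UI widgets, then after a short delay loads high scores, settings and customization.
; LoadLevel configures the AI spawner and shift timer from CurrentLevelInfo while async loading, and BoxDead ends the shift early once all boxes are used.
; LoadMenu restores menu input and music, resets both characters and saves.
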(event Custom|Save
  ;[0.15 0.15 0.15 0.5] Save score data
  (bind _output_get (Variables|Default|SetSaveState (Utilities|Struct|MakeGameData (Variables|/Script/SpmG5.ScoreManager|GetScoreMap (Subsystems|GetScoreManager)) (.MasterVolume (Utilities|Struct|BreakGameData (Variables|Default|GetSaveState))) (.MusicVolume (Utilities|Struct|BreakGameData (Variables|Default|GetSaveState))) (.SFXVolume (Utilities|Struct|BreakGameData (Variables|Default|GetSaveState))) (.StopCameraMove (Utilities|Struct|BreakGameData (Variables|Default|GetSaveState))) (.Player0CustomizationIndex (Utilities|Struct|BreakGameData (Variables|Default|GetSaveState))) (.Player1CustomizationIndex (Utilities|Struct|BreakGameData (Variables|Default|GetSaveState))))))
  (Class|SaveManager|SaveGame _output_get))

(event Custom|Load%20Data
  ;[0.15 0.15 0.15 0.5] Load score data
  (bind _returnvalue (Class|SaveManager|LoadGame))
  (bind _output_get (Variables|Default|SetSaveState _returnvalue))
  (Class|ScoreManager|SetAllHighScores (Subsystems|GetScoreManager) (.HighScores (Utilities|Struct|BreakGameData _output_get)))
  (Default|LoadSettings (Variables|Default|GetSettings))
  (Default|LoadCustomization (Variables|Default|GetMenu)))

(event Custom|LoadMenu
  (bind (_player_character_1 _player_character_2) (CallFunction|GetPlayerCharacter))
  (bind (_customcontroller1 _customcontroller2) (CallFunction|GetGameController))
  (bind _menu (Variables|Default|GetMenu))
  (bind _menu_2 (Variables|Default|GetMenu))
  ;[0.15 0.15 0.15 0.5] Loads menu
  (Variables|Default|SetCanBoxDead false)
  (Variables|Default|SetCanPause false)
  (Class|ScoreManager|SaveScore (Subsystems|GetScoreManager))
  (Default|UpdateHighscoreUI _menu_2)
  (UserInterface|Viewport|AddtoViewport _menu_2 0)
  (Variables|Default|SetbIsInLevel false)
  (|LoadLevelAsync "/Game/Levels/Menu.Menu"
    (:then
      (Widget|RemovefromParent (Variables|Default|GetHud)))
    (:OnLevelLoaded
      (Variables|/Script/Engine.PlayerController|SetbShowMouseCursor _customcontroller1 true)
      (Input|SetInputModeUIOnly _customcontroller1 _menu "DoNotLock" true)
      (Input|SetInputModeUIOnly _customcontroller2 _menu "DoNotLock" true)
      (bind _returnvalue (Class|FMODBlueprintStatics|PlayEvent2D "/Game/FMOD/Events/Music/Mu_MainMenu.Mu_MainMenu"))
      (Variables|Default|SetMusicInstance _returnvalue)
      (Default|ResetCharacter _player_character_1)
      (Default|ResetCharacter _player_character_2)
      (CallFunction|Save))))

(event Custom|OpenSettings
  (Utilities|FlowControl|FlipFlop
    (:A
      (CallFunction|ShowSettings))
    (:B
      (CallFunction|CloseSettings))))

(event Custom|Load%20Level
  (bind _customcontroller1 (CallFunction|GetGameController))
  (bind _startcountdown (Variables|Default|GetStartCountdown))
  (bind _currentlevelinfo (Variables|Default|GetCurrentLevelInfo))
  (bind _currentlevelinfo_2 (Variables|Default|GetCurrentLevelInfo))
  (bind _currentlevelinfo_3 (Variables|Default|GetCurrentLevelInfo))
  (bind (_level _pointstopass _shifttime _levelname _istutorial _bshowinstructionswidget _instructionsimage _amountofboxesperlevel _spawnrates _dangeroustypes _boxaddresses) (Utilities|Struct|BreakLevelInfo _currentlevelinfo_2))
  (bind (_level_2 _pointstopass_2 _shifttime_2 _levelname_2 _istutorial_2 _bshowinstructionswidget_2) (Utilities|Struct|BreakLevelInfo _currentlevelinfo_3))
  (bind (_level_3 _pointstopass_3 _shifttime_3 _levelname_3 _istutorial_3 _bshowinstructionswidget_3 _instructionsimage_2 _amountofboxesperlevel_2) (Utilities|Struct|BreakLevelInfo _currentlevelinfo))
  ;[0.15 0.15 0.15 0.5] Loads level from level button
  (Class|SpawnAI|SetupSpawner (Subsystems|GetSpawnAI) _amountofboxesperlevel _spawnrates _dangeroustypes _boxaddresses)
  (CallFunction|InitMusic)
  (CallFunction|SetupLevel)
  (|LoadLevelAsync _level_2
    (:then
      (Widget|RemovefromParent (Variables|Default|GetMenu))
      (Widget|RemovefromParent (Variables|Default|GetInstructionWidget))
      (Widget|RemovefromParent (Variables|Default|GetWinOrLoseWidget)))
    (:OnLevelLoaded
      (Variables|Default|SetLevelCameraLocation (Camera|GetCameraLocation (Game|GetPlayerCameraManager 0)))
      (Utilities|FlowControl|Delay 0.2)
      (if _bshowinstructionswidget_2
        (UserInterface|Viewport|AddtoViewport (Variables|Default|GetInstructionWidget) 0)
        (CallFunction|Pause)
        (Utilities|FlowControl|Delay 3.0)
        (Widget|RemovefromParent (Variables|Default|GetInstructionWidget)))
      (if _istutorial_2
        _
        (else
          (UserInterface|Viewport|AddtoViewport _startcountdown 0)
          (Default|PlayCountdown _startcountdown)))
      (Variables|/Script/Engine.PlayerController|SetbShowMouseCursor (.CustomController1 (CallFunction|GetGameController)) false)
      (Variables|Default|SetbIsInLevel true)
      (Variables|Default|SetUsedBoxes 0)
      (Variables|Default|SetTotalBoxes _amountofboxesperlevel_2)
      (Variables|Default|SetCanBoxDead true)
      (if _istutorial_3
        (Input|SetInputModeGameandUI _customcontroller1 0 "DoNotLock" true false)
        (else
          (Input|SetInputModeGameOnly _customcontroller1 false))))))

(event EventPauseGame
  (CallFunction|Pause))

(event EventBoxDead
  ;[0.15 0.15 0.15 0.5] End level if no boxes
  (if (Variables|Default|GetCanBoxDead)
    (Math|Integer|IncrementInt (Variables|Default|GetUsedBoxes)
      (:%20%20
        (if (>= (Variables|Default|GetUsedBoxes) (Variables|Default|GetTotalBoxes))
          (Class|ShiftManager|EndShiftEarly (Subsystems|GetShiftManager)))))))

(event EventInit
  ;[0.15 0.15 0.15 0.5] Loads all necessary widgets
  (Utilities|FlowControl|Sequence
    (:then_0
      (bind _returnvalue (UserInterface|CreateWidget "/Game/Widgets/WBP_HUD.WBP_HUD_C"))
      (Variables|Default|SetHud _returnvalue)
      (bind _returnvalue_2 (UserInterface|CreateWidget "/Game/Widgets/WBP_Menu.WBP_Menu_C"))
      (Variables|Default|SetMenu _returnvalue_2)
      (bind _returnvalue_3 (UserInterface|CreateWidget "/Game/Widgets/WBP_InstructionFlowChart.WBP_InstructionFlowChart_C"))
      (Variables|Default|SetInstructionWidget _returnvalue_3)
      (bind _returnvalue_4 (UserInterface|CreateWidget "/Game/Widgets/WBP_ControllerMap.WBP_ControllerMap_C"))
      (Variables|Default|SetControllerWidget _returnvalue_4))
    (:then_1
      (bind _returnvalue_5 (UserInterface|CreateWidget "/Game/Widgets/WBP_WinOrLoseScreen.WBP_WinOrLoseScreen_C"))
      (Variables|Default|SetWinOrLoseWidget _returnvalue_5)
      (bind _returnvalue_6 (UserInterface|CreateWidget "/Game/Widgets/WBP_Pause.WBP_Pause_C"))
      (Variables|Default|SetPauseWidget _returnvalue_6)
      (bind _returnvalue_7 (UserInterface|CreateWidget "/Game/Widgets/WBP_Settings.WBP_Settings_C"))
      (Variables|Default|SetSettings _returnvalue_7))
    (:then_2
      (bind _returnvalue_8 (UserInterface|CreateWidget "/Game/Widgets/WBP_StartLevelCountdown.WBP_StartLevelCountdown_C"))
      (Variables|Default|SetStartCountdown _returnvalue_8)
      (bind _returnvalue_9 (UserInterface|CreateWidget "/Game/Widgets/WBP_ResultScreen.WBP_ResultScreen_C"))
      (Variables|Default|SetResultsWidget _returnvalue_9))
    (:then_3
      ;[0.15 0.15 0.15 0.5] Load save data
      (Utilities|FlowControl|Delay 0.2)
      (CallFunction|LoadData)
      (Default|UpdateHighscoreUI (Variables|Default|GetMenu)))))

(fn Pause
  (bind _customcontroller1 (CallFunction|GetGameController))
  (bind _pausewidget (Variables|Default|GetPauseWidget))
  (if (Variables|Default|GetCanPause)
    (Game|SetGamePaused (Class|KismetMathLibrary|XORBoolean (Game|IsGamePaused) true))
    (if (Game|IsGamePaused)
      (UserInterface|Viewport|AddtoViewport _pausewidget 0)
      (Input|SetInputModeGameandUI _customcontroller1 _pausewidget "DoNotLock" true false)
      (else
        (Widget|RemovefromParent _pausewidget)
        (Input|SetInputModeGameOnly _customcontroller1 false)))
    (Variables|/Script/Engine.PlayerController|SetbShowMouseCursor (.CustomController1 (CallFunction|GetGameController)) (Game|IsGamePaused))))

(fn ShowSettings
  (bind _settings (Variables|Default|GetSettings))
  (Widget|RemovefromParent (Variables|Default|GetPauseWidget))
  (UserInterface|Viewport|AddtoViewport _settings 0)
  (Input|SetInputModeGameandUI (.CustomController1 (CallFunction|GetGameController)) _settings "DoNotLock" true false))

(fn CloseSettings
  (bind _pausewidget (Variables|Default|GetPauseWidget))
  (Widget|RemovefromParent (Variables|Default|GetSettings))
  (UserInterface|Viewport|AddtoViewport _pausewidget 0)
  (Input|SetInputModeGameandUI (.CustomController1 (CallFunction|GetGameController)) _pausewidget "DoNotLock" true false)
  (Development|PrintString "razzclat"))

(fn InitMusic
  (bind _musicinstance (Variables|Default|GetMusicInstance))
  (bind _returnvalue (Class|FMODBlueprintStatics|EventInstanceIsValid _musicinstance))
  (if _returnvalue
    (Class|FMODBlueprintStatics|EventInstanceStop _musicinstance false)))

(fn SetupLevel
  (bind _currentlevelinfo (Variables|Default|GetCurrentLevelInfo))
  (bind _hud (Variables|Default|GetHud))
  (bind (_level _pointstopass _shifttime _levelname _istutorial) (Utilities|Struct|BreakLevelInfo _currentlevelinfo))
  (Class|ShiftManager|SetShiftTime (Subsystems|GetShiftManager) _shifttime)
  (if (not _istutorial)
    (if (UserInterface|Viewport|IsinViewport (Variables|Default|GetHud))
      _
      (else
        (UserInterface|Viewport|AddtoViewport _hud 0)))
    (Default|SetStartTime _hud (.ShiftTime (Utilities|Struct|BreakLevelInfo (Variables|Default|GetCurrentLevelInfo))))
    (Class|ShiftManager|StartTimer (Subsystems|GetShiftManager))))