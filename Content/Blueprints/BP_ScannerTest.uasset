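; BP_ScannerTest is a test scanner actor that reports whether the package a player carries is dangerous.
; When a BP_CustomCharacter overlaps it, it binds Scan to that character's interact dispatcher and unbinds it on end overlap.
; Scan checks whether the character holds an item, then prints a red DANGEROUS or green GOOD message from the item's IsDangerous flag, or a no-box message.
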(event Custom|Scan
  (Development|PrintString "Box is scanning")
  (bind _returnvalue (Class|SpmG5Character|GetHasItem (stale Collision|EventActorBeginOverlap _asbp_custom_character)))
  (if _returnvalue
    (Development|PrintString "yes")
    (bind _returnvalue_2 (Class|SpmG5Character|GetItem (stale Collision|EventActorBeginOverlap _asbp_custom_character)))
    (if (Class|Item|GetIsDangerous _returnvalue_2)
      (Development|PrintString "This package is DANGEROUS" true true "(R=1.000000,G=0.084021,B=0.000000,A=1.000000)")
      (else
        (Development|PrintString "This package is GOOD" true true "(R=0.143894,G=1.000000,B=0.206475,A=1.000000)")))
    (else
      (Development|PrintString "no box"))))

(event Collision|EventActorBeginOverlap
  (params (OtherActor :type Actor%20Object%20Reference))
  (bind _asbp_custom_character (Utilities|Casting|CastToBP_CustomCharacter OtherActor))
  (Development|PrintString "bro is overlapping")
  (EventDispatchers|BindEventtoInteractDispatcher _asbp_custom_character (delegate Custom|Scan)))

(event Collision|EventActorEndOverlap
  (params (OtherActor :type Actor%20Object%20Reference))
  (Utilities|Casting|CastToBP_CustomCharacter OtherActor)
  (Development|PrintString "Bro left ;(")
  (EventDispatchers|UnbindEventfromInteractDispatcher (stale Collision|EventActorBeginOverlap _asbp_custom_character) (delegate Custom|Scan)))

(fn ConstructionScript)