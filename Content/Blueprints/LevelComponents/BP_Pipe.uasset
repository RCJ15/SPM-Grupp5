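; BP_Pipe is a level hazard pipe that blows wind at players and items, with a child alarm light for indication.
; ShowIndication turns on the lamp, and ActivateBlowing toggles the wind VFX, clearing the alarm when blowing stops.
; Each blowing call runs one box trace, ragdolling and launching a hit character or pushing a hit Item along the pipe's forward vector.
; Force strength is cached at BeginPlay.
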(event EventBeginPlay
  ;[0.15 0.15 0.15 0.5] New Blowing
  (bind _returnvalue (Class|BlowPipe|GetForceMultiplier))
  (Variables|Default|SetForceMult _returnvalue)
  (bind _asbp_alarm_light (Utilities|Casting|CastToBP_AlarmLight (Variables|/Script/Engine.ChildActorComponent|GetChildActor (Variables|Default|GetBP_AlarmLight))))
  (Variables|Default|SetLamp _asbp_alarm_light))

(event Collision|EventActorBeginOverlap
  (params (OtherActor :type Actor%20Object%20Reference)))

(event EventTick
  (params (DeltaSeconds :type Float%20%28single-precision%29)))

(event EventActivateBlowing
  (params (Blowing :type Boolean))
  (bind _returnvalue (Transformation|GetActorLocation))
  (bind _returnvalue_2 (Transformation|GetActorForwardVector))
  (bind _windvfx (Variables|Default|GetWindVFX))
  (bind _blowarea (Variables|Default|GetBlowArea))
  (bind _arrow (Variables|Default|GetArrow))
  (bind _forcemult (Variables|Default|GetForceMult))
  (bind _returnvalue_3 (Transformation|GetSocketLocation _arrow "None"))
  (bind _returnvalue_4 (Transformation|GetSocketLocation _blowarea "None"))
  (bind _returnvalue_5 (* _returnvalue_2 _forcemult))
  (bind _returnvalue_6 (- _returnvalue_3 _returnvalue_4))
  (bind _returnvalue_7 (* _returnvalue_6 -1))
  (bind _returnvalue_8 (+ _returnvalue_7 _returnvalue))
  ;[0.15 0.15 0.15 0.5] New Blowing
  (if Blowing
    (Components|Activation|Activate _windvfx false)
    (bind _outhit (Collision|BoxTraceByChannel _returnvalue_8 _returnvalue_8 (Components|Box|GetScaledBoxExtent (Variables|Default|GetBlowArea)) (Transformation|GetActorRotation) "TraceTypeQuery6" false 0 "ForOneFrame"))
    (bind _asspm_g5character (Utilities|Casting|CastToSpmG5Character (.HitActor (Collision|BreakHitResult _outhit)))
      (:then
        (Class|SpmG5Character|DoRagdoll _asspm_g5character)
        (Character|LaunchCharacter _asspm_g5character (Math|Vector|MakeVector (.x _returnvalue_5) (.y _returnvalue_5) 5e+01) true true))
      (:CastFailed
        (bind _asitem (Utilities|Casting|CastToItem (.HitActor (Collision|BreakHitResult _outhit))))
        (Physics|AddForce (Variables|/Script/SpmG5.Item|GetBaseMesh _asitem) (* (* (Transformation|GetActorForwardVector) 1000) (Variables|Default|GetForceMult)) "None" false)))
    (else
      (Components|Activation|Deactivate _windvfx)
      (Default|FSetAlarmActive (Variables|Default|GetLamp) false))))

(event EventShowIndication
  (Default|FSetAlarmActive (Variables|Default|GetLamp) true))

(fn ConstructionScript)