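; Interactable parcel scanner that checks whether an already-scanned package is dangerous.
; Interacting moves the player's held item into the box, where a timeline sweeps the scanner mesh down with an attached FMOD sound.
; When finished, a DangerousItem cast picks the cross or checkmark icon on a UI plane and sets the sound's Success parameter.
; Interacting again returns the item, while invalid or busy attempts briefly show a status icon.
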(event EventOnInteract
  (params (InteractingPlayer :type Spm%20G5%20Character%20Object%20Reference))
  (bind _scanstart (Variables|Default|GetScanStart))
  (bind _returnvalue (Transformation|GetRelativeTransform _scanstart))
  (bind _location (Math|Transform|BreakTransform _returnvalue))
  (bind (_x _y _z) (Math|Vector|BreakVector _location))
  (Variables|Default|SetInteracting%20Player InteractingPlayer)
  (Utilities|IsValid (Variables|Default|GetScanningItem)
    (:Is%20Valid
      (if (Variables|Default|GetisScanning)
        (Development|PrintString "box is busy")
        ;[0.15 0.15 0.15 0.5] Visar UI resultat
        (Rendering|Material|SetMaterial (Variables|Default|GetUIPlane) 0 "/Game/UI/M_IconAlreadyFullGreen.M_IconAlreadyFullGreen")
        (Rendering|SetVisibility (Variables|Default|GetUIPlane) true false :!label _label)
        (Utilities|FlowControl|Delay 1.5)
        (Rendering|SetVisibility (Variables|Default|GetUIPlane) false false)
        (else
          (Transformation|DetachFromActor (Variables|Default|GetScanningItem) "KeepRelative" "KeepRelative" "KeepRelative")
          (Class|SpmG5Character|Pickup (Variables|Default|GetInteracting%20Player) (Variables|Default|GetScanningItem))
          (Variables|Default|SetScanningItem 0)
          (bind _output_get (Variables|Default|SetVisibility false))
          (Rendering|SetVisibility (Variables|Default|GetUIPlane) _output_get false))))
    (:Is%20Not%20Valid
      (if (Class|SpmG5Character|GetHasItem (Variables|Default|GetInteracting%20Player))
        (if (Class|Item|GetIsScanned (Class|SpmG5Character|GetItem (Variables|Default|GetInteracting%20Player)))
          (Variables|Default|SetisScanning true)
          (bind _returnvalue_2 (Class|SpmG5Character|Drop (Variables|Default|GetInteracting%20Player)))
          (Variables|Default|SetScanningItem _returnvalue_2)
          ;[0.15 0.15 0.15 0.5] Start SFX and stop if SFX already exists - Ruben
          (if (Utilities|IsValid (Variables|Default|GetFMOD%20SFX))
            (Class|FMODAudioComponent|Stop (Variables|Default|GetFMOD%20SFX)))
          (bind _returnvalue_3 (Class|FMODBlueprintStatics|PlayEventAttached "/Game/FMOD/Events/SFX/Stations/SFX_Scanner.SFX_Scanner" (Variables|Default|GetBoxHolder) "None" "0, 0, 0" "KeepRelativeOffset"))
          (Variables|Default|SetFMOD%20SFX _returnvalue_3)
          (Transformation|AttachComponentToComponent (Variables|Default|GetScanningItem) (Variables|Default|GetBoxHolder) "None" "SnapToTarget" "SnapToTarget" "KeepRelative" true)
          (Rendering|SetVisibility (Variables|Default|GetSM_ParcelScanner) true false)
          (bind _duration (Timeline|Timeline PlayFromStart)
            (:Update
              (Class|MovieSceneTransformOrigin|GetTransformOrigin(Message) (Variables|Default|GetSM_ParcelScanner))
              (Transformation|SetRelativeTransform (Variables|Default|GetSM_ParcelScanner) (Math|Conversions|ToTransform(Vector) (Math|Vector|MakeVector _x _y (Math|Float|Lerp _z (.Z (Math|Vector|BreakVector (.Location (Math|Transform|BreakTransform (Transformation|GetRelativeTransform (Variables|Default|GetScanBottom)))))) _duration))) false false))
            (:Finished
              (Rendering|SetVisibility (Variables|Default|GetSM_ParcelScanner) false false)
              (Variables|Default|SetisScanning false)
              (Variables|Default|SetVisibility true)
              (Utilities|Casting|CastToDangerousItem (Variables|Default|GetScanningItem)
                (:then
                  (Development|PrintString "This package is BAD" true true "(R=1.000000,G=0.084021,B=0.000000,A=1.000000)")
                  ;[0.15 0.15 0.15 0.5] Set SFX parameter - Ruben
                  (Class|FMODAudioComponent|SetParameter (Variables|Default|GetFMOD%20SFX) "Success" 0.0)
                  ;[0.15 0.15 0.15 0.5] Visar UI resultat
                  (Rendering|Material|SetMaterial (Variables|Default|GetUIPlane) 0 "/Game/UI/M_IconCross.M_IconCross"))
                (:CastFailed
                  (Development|PrintString "This package is GOOD" true true "(R=0.143894,G=1.000000,B=0.206475,A=1.000000)")
                  (Class|FMODAudioComponent|SetParameter (Variables|Default|GetFMOD%20SFX) "Success" 1.0)
                  (Rendering|Material|SetMaterial (Variables|Default|GetUIPlane) 0 "/Game/UI/M_IconCheckmark.M_IconCheckmark")))
              (Rendering|SetVisibility (Variables|Default|GetUIPlane) (Variables|Default|GetVisibility) false)
              ;[0.15 0.15 0.15 0.5] Stop SFX and set it to null - Ruben
              (Class|FMODAudioComponent|Stop (Variables|Default|GetFMOD%20SFX))
              (Variables|Default|SetFMOD%20SFX 0)))
          (else
            (Development|PrintString "Scan your box first.")
            (Rendering|Material|SetMaterial (Variables|Default|GetUIPlane) 0 "/Game/UI/M_IconScanFirst.M_IconScanFirst")
            (goto _label)))
        (else
          (Development|PrintString "no box")
          (Rendering|Material|SetMaterial (Variables|Default|GetUIPlane) 0 "/Game/UI/M_IconNeedBox.M_IconNeedBox")
          (goto _label))))))

(fn ConstructionScript)