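; BP_Door is a toggleable door that opens by shrinking its static mesh along the Y axis rather than moving or rotating it.
; DoorInteraction flips IsOpen and plays a timeline forward or in reverse, lerping the Y scale between full size and zero.
; CanClick blocks further interaction until the timeline finishes.
; BeginPlay collapses the mesh immediately when the door starts open.
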(event Custom|DoorInteraction
  (if (Variables|Default|GetcanClick)
    (Variables|Default|SetcanClick false)
    (if (Variables|Default|GetisOpen)
      (Variables|Default|SetisOpen false)
      (bind _door (Timeline|Timeline ReverseFromEnd)
        (:Update
          (Transformation|SetRelativeScale3D (Variables|Default|GetStaticMesh) (Math|Vector|MakeVector 0.4 (Math|Float|Lerp 2.0 0.0 _door) 2.0)))
        (:Finished
          (Variables|Default|SetcanClick true)))
      (else
        (Variables|Default|SetisOpen true)
        (Timeline|Timeline PlayFromStart)))))

(event EventBeginPlay
  (if (Variables|Default|GetisOpen)
    (Transformation|SetRelativeScale3D (Variables|Default|GetStaticMesh) "0.400000,0.000000,2.000000")))

(fn ConstructionScript)