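; BP_Getters is a set of shared lookup functions that return the game manager, controllers and characters for a two-player game.
; The game manager comes from the Game Instance, and the two custom controllers come from player indices 0 and 1.
; Character lookup feeds each controller's ID into Get Player Pawn as the player index.
; Every result is cast to its project class, and a failed cast halts that getter.
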(fn GetGameManager
  (bind _asbp_game_manager (Utilities|Casting|CastToBP_GameManager (Game|GetGameInstance (LocalVariables|Get__WorldContext))))
  (return _asbp_game_manager))

(fn GetGameController
  (bind _asbp_custom_controller (Utilities|Casting|CastToBP_CustomController (Game|GetPlayerController 0 1)))
  (bind _asbp_custom_controller_2 (Utilities|Casting|CastToBP_CustomController (Game|GetPlayerController 0)))
  (return _asbp_custom_controller_2 _asbp_custom_controller))

(fn GetPlayerCharacter
  (bind ___worldcontext (LocalVariables|Get__WorldContext))
  (bind (_customcontroller1 _customcontroller2) (CallFunction|GetGameController ___worldcontext))
  (bind _asbp_custom_character (Utilities|Casting|CastToBP_CustomCharacter (Game|Player|GetPlayerPawn 0 (Class|GameplayStatics|GetPlayerControllerID _customcontroller2))))
  (bind _asbp_custom_character_2 (Utilities|Casting|CastToBP_CustomCharacter (Game|Player|GetPlayerPawn 0 (Class|GameplayStatics|GetPlayerControllerID _customcontroller1))))
  (return _asbp_custom_character_2 _asbp_custom_character))