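; BP_Door is a sliding door that toggles open and closed through its DoorInteraction event, with whirr and close sounds attached to the mesh.
; A timeline plays forward to open or in reverse to close, with CanClick blocking input until it finishes.
; Each update lerps the mesh's relative location from the actor's world location along X or Y, chosen by IsVertical, with the offset sign depending on IsOpen.
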(event Custom|DoorInteraction
  (bind _returnvalue (Transformation|GetActorLocation))
  (bind _returnvalue_2 (Transformation|GetActorLocation))
  (bind _returnvalue_3 (Transformation|GetActorLocation))
  (bind _returnvalue_4 (Transformation|GetActorLocation))
  (if (Variables|Default|GetcanClick)
    (Class|FMODBlueprintStatics|PlayEventAttached "/Game/FMOD/Events/SFX/Door/SFX_DoorWhirr.SFX_DoorWhirr" (Variables|Default|GetStaticMesh) "None" "0, 0, 0" "KeepRelativeOffset")
    (Variables|Default|SetcanClick false)
    (if (Variables|Default|GetisOpen)
      (Variables|Default|SetisOpen false)
      (bind _door (Timeline|Timeline ReverseFromEnd)
        (:Update
          (if (Variables|Default|GetisVertical)
            ;[0.15 0.15 0.15 0.5] Viktor FIx
            (if (Variables|Default|GetisOpen)
              (Transformation|SetRelativeLocation (Variables|Default|GetStaticMesh) (Math|Vector|MakeVector (Math|Float|Lerp (.x _returnvalue) (+ (.x _returnvalue) 5.7) _door) (.y _returnvalue) (.z _returnvalue)) false false)
              (else
                (Transformation|SetRelativeLocation (Variables|Default|GetStaticMesh) (Math|Vector|MakeVector (Math|Float|Lerp (.x _returnvalue_2) (- (.x _returnvalue_2) 5.7) _door) (.y _returnvalue_2) (.z _returnvalue_2)) false false)))
            (else
              ;[0.15 0.15 0.15 0.5] Marcus spaget
              (if (Variables|Default|GetisOpen)
                (Transformation|SetRelativeLocation (Variables|Default|GetStaticMesh) (Math|Vector|MakeVector (.x _returnvalue_3) (Math|Float|Lerp (.y _returnvalue_3) (- (.y _returnvalue_3) 5.4) _door) (.z _returnvalue_3)) false false)
                (else
                  (Transformation|SetRelativeLocation (Variables|Default|GetStaticMesh) (Math|Vector|MakeVector (.x _returnvalue_4) (Math|Float|Lerp (.y _returnvalue_4) (+ (.y _returnvalue_4) 5.4) _door) (.z _returnvalue_4)) false false))))))
        (:Finished
          (Variables|Default|SetcanClick true)
          (Class|FMODBlueprintStatics|PlayEventAttached "/Game/FMOD/Events/SFX/Door/SFX_DoorClose.SFX_DoorClose" (Variables|Default|GetStaticMesh) "None" "0, 0, 0" "KeepRelativeOffset")))
      (else
        (Variables|Default|SetisOpen true)
        (Timeline|Timeline PlayFromStart)))))

(fn ConstructionScript)