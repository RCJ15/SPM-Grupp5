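; BP_RadioactiveItem is a radioactive item that affects characters standing within its radius.
; Begin and end overlap events on RadioactiveRadius switch IncreaseIncapacitation on and off for any SpmG5Character, printing a debug string each time.
; An author note says carrying the item makes the overlap toggle rapidly because the object teleports, pending a new carry implementation.
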(event OnComponentBeginOverlap(RadioactiveRadius)
  (params (OverlappedComponent :type Primitive%20Component%20Object%20Reference) (OtherActor :type Actor%20Object%20Reference) (OtherComp :type Primitive%20Component%20Object%20Reference) (OtherBodyIndex :type Integer) (bFromSweep :type Boolean) (SweepResult :type Hit%20Result%20Structure%20%28by%20ref%29))
  ;[0.15 0.15 0.15 0.5] Detta spammas av och på när man går runt med objektet då objektet teleporteras, men det bör bli löst när nya bär versionen implementeras
  (bind _asspm_g5character (Utilities|Casting|CastToSpmG5Character OtherActor))
  (Development|PrintString "START OVERLAP RADIOACTIVE")
  (Variables|/Script/SpmG5.SpmG5Character|SetbIncreaseIncapacitation _asspm_g5character true))

(event OnComponentEndOverlap(RadioactiveRadius)
  (params (OverlappedComponent :type Primitive%20Component%20Object%20Reference) (OtherActor :type Actor%20Object%20Reference) (OtherComp :type Primitive%20Component%20Object%20Reference) (OtherBodyIndex :type Integer))
  ;[0.15 0.15 0.15 0.5] Detta spammas av och på när man går runt med objektet då objektet teleporteras, men det bör bli löst när nya bär versionen implementeras
  (bind _asspm_g5character (Utilities|Casting|CastToSpmG5Character OtherActor))
  (Development|PrintString "STOP OVERLAP RADIOACTIVE")
  (Variables|/Script/SpmG5.SpmG5Character|SetbIncreaseIncapacitation _asspm_g5character false))

(event EventBeginPlay
  (|CallParentFunction) ; This node is disabled and will not be called.\nDrag off pins to build functionality.
)

(event Collision|EventActorBeginOverlap
  (params (OtherActor :type Actor%20Object%20Reference)))

(event EventTick
  (params (DeltaSeconds :type Float%20%28single-precision%29)))

(fn ConstructionScript
  (|CallParentFunction))