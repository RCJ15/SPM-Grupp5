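; BP_SpawnAI holds a SpawnRates map keyed by type, apparently for spawn configuration, but contains no spawning logic.
; The construction script loops over the map and, on finding a Bomb key, removes it and adds Small at a zero rate, modifying the map during iteration.
; The event graph holds only disabled stubs, and leftover small/large box percentage math never runs.
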(event EventBeginPlay)

(event Collision|EventActorBeginOverlap
  (params (OtherActor :type Actor%20Object%20Reference)))

(event EventTick
  (params (DeltaSeconds :type Float%20%28single-precision%29)))

(fn ConstructionScript
  (bind _spawnrates (Variables|Default|GetSpawnRates))
  (bind _keypin (Utilities|Map|ForEachLoop(Map) (Variables|Default|GetSpawnRates))
    (:then
      (if (Utilities|Enum|Equal(Enum) _keypin "Bomb")
        (Utilities|Map|Remove _spawnrates "Bomb")
        (Utilities|Map|Add _spawnrates "Small" 0.0)))))