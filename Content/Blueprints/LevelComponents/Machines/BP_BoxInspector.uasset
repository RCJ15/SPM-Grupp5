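; Parcel inspection station that takes a pre-scanned item by interact, swap or throw, and reveals whether it is good or bad.
; A timeline grows a scan dome, then after a delay the item gains points and a decal, and bad bombs start their countdown.
; A camera-facing icon plane, parcel meshes and FMOD audio report status and results.
; The machine can break, blocking new items until a player completes a cancellable timed repair.
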(event OnComponentHit(StaticMesh)
  (params (HitComponent :type Primitive%20Component%20Object%20Reference) (OtherActor :type Actor%20Object%20Reference) (OtherComp :type Primitive%20Component%20Object%20Reference) (NormalImpulse :type Vector :default "0, 0, 0") (Hit :type Hit%20Result%20Structure%20%28by%20ref%29))
  (bind _scanningitem (Variables|Default|GetScanningItem))
  (bind _scanningitem_2 (Variables|Default|GetScanningItem))
  (bind _returnvalue (Actor|GetComponentbyClass _scanningitem "/Script/Engine.DecalComponent"))
  ;[0.15 0.15 0.15 0.5] Så man kan kasta in items i stationen!
  (if (not (Variables|Default|GetIsBroken))
    (bind _asitem (Utilities|Casting|CastToItem OtherActor))
    (bind _shouldcontinue (CallFunction|HandleThrow _asitem))
    (if _shouldcontinue
      (Variables|/Script/SpmG5.Item|SetbIsInStation (Variables|Default|GetScanningItem) true)
      (CallFunction|StartSFX)
      (Transformation|AttachComponentToComponent (Variables|Default|GetScanningItem) (Variables|Default|GetBoxHolder) "None" "SnapToTarget" "SnapToTarget" "KeepRelative" true)
      (Rendering|SetVisibility (Variables|Default|GetSM_ScanDome) true false)
      (Rendering|SetVisibility (Variables|Default|GetScanDecal) true false)
      (bind _alpha (Timeline|ScanDomeScale PlayFromStart)
        (:Update
          (Transformation|SetRelativeScale3D (Variables|Default|GetSM_ScanDome) (Math|Vector|Lerp(Vector) "0.010000,0.010000,0.010000" "7.375000,7.375000,8.000000" _alpha)))
        (:Finished
          (Rendering|SetVisibility (Variables|Default|GetScanDecal) false false)
          (Rendering|SetVisibility (Variables|Default|GetSM_ScanDome) false false)
          (Niagara|SpawnSystematLocation "/Game/VFX/NS_UnpackingSmoke.NS_UnpackingSmoke" (Transformation|GetWorldLocation (Variables|Default|GetUnpackSmokeSpawn)))
          (Utilities|FlowControl|Delay (Variables|Default|GetDuration))
          (Variables|Default|SetisScanning false)
          (Utilities|IsValid _scanningitem_2
            (:Is%20Valid
              (Class|Item|SetIsInspected _scanningitem_2 true)
              (Class|Item|AddBonusPoints _scanningitem_2 (Variables|/Script/SpmG5.Item|GetInspectedPoints _scanningitem_2))
              (Variables|Default|SetVisibility true)
              (if (CallFunction|GetIsBadItem (Variables|Default|GetScanningItem))
                (bind _asdangerous_item (Utilities|Casting|CastToDangerousItem (Variables|Default|GetScanningItem))
                  (:then
                    _)
                  (:CastFailed
                    _))
                ;[0.15 0.15 0.15 0.5] visa X dekal
                (Rendering|Components|Decal|SetDecalMaterial _returnvalue "/Game/UI/Items/M_Decal_AddressXmark.M_Decal_AddressXmark")
                (Rendering|SetVisibility _returnvalue (not (Utilities|IsValid _asdangerous_item)) false)
                (bind _asbp_bomb (Utilities|Casting|CastToBP_Bomb (Variables|Default|GetScanningItem))
                  (:then
                    (Default|BecomeABomb _asbp_bomb)
                    (Class|DangerousItem|StartCountDownTimer _asbp_bomb))
                  (:CastFailed
                    _))
                (Development|PrintString "This package is BAD" true true "(R=1.000000,G=0.084021,B=0.000000,A=1.000000)")
                ;[0.15 0.15 0.15 0.5] Set SFX parameter - Ruben
                (Class|FMODAudioComponent|SetParameter (Variables|Default|GetFMOD%20SFX) "Success" 0.0)
                ;[0.15 0.15 0.15 0.5] Visar UI resultat
                (Rendering|Material|SetMaterial (Variables|Default|GetUIPlane) 0 "/Game/UI/Popups/M_IconCross.M_IconCross")
                (Rendering|SetVisibility (Variables|Default|GetParcelBad) true false)
                (else
                  ;[0.15 0.15 0.15 0.5] Gå från att visa ? dekal till address dekal
                  (Class|Item|SetAddressDecal (Variables|Default|GetScanningItem))
                  ;[0.15 0.15 0.15 0.5] visa dekal
                  (Rendering|SetVisibility (Actor|GetComponentbyClass (Variables|Default|GetScanningItem) "/Script/Engine.DecalComponent") true false)
                  (Development|PrintString "This package is GOOD" true true "(R=0.143894,G=1.000000,B=0.206475,A=1.000000)")
                  (Class|FMODAudioComponent|SetParameter (Variables|Default|GetFMOD%20SFX) "Success" 1.0)
                  (Rendering|Material|SetMaterial (Variables|Default|GetUIPlane) 0 "/Game/UI/Popups/M_IconCheckmark.M_IconCheckmark")
                  (Rendering|SetVisibility (Variables|Default|GetParcelGood) true false)))
              (Rendering|SetVisibility (Variables|Default|GetUIPlane) (Variables|Default|GetVisibility) false)
              ;[0.15 0.15 0.15 0.5] Stop SFX and set it to null - Ruben
              (Class|FMODAudioComponent|Stop (Variables|Default|GetFMOD%20SFX))
              (Variables|Default|SetFMOD%20SFX 0)
              (Variables|Default|SetTempHeldItem 0))))))))

(event EventOnInteract
  (params (InteractingPlayer :type Spm%20G5%20Character%20Object%20Reference))
  (Variables|Default|SetInteracting%20Player InteractingPlayer)
  (Utilities|IsValid (Variables|Default|GetScanningItem)
    (:Is%20Valid
      (if (Variables|Default|GetisScanning)
        (Development|PrintString "box is busy")
        ;[0.15 0.15 0.15 0.5] Visar UI resultat
        (Rendering|Material|SetMaterial (Variables|Default|GetUIPlane) 0 "/Game/UI/Popups/M_IconAlreadyFullGreen.M_IconAlreadyFullGreen")
        (Rendering|SetVisibility (Variables|Default|GetUIPlane) true false :!label _label)
        (Utilities|FlowControl|Delay 1.5)
        (Rendering|SetVisibility (Variables|Default|GetUIPlane) false false)
        (elif (Class|SpmG5Character|GetHasItem (Variables|Default|GetInteracting%20Player))
          ;[0.15 0.15 0.15 0.5] Swap items
          (if (and (Class|Item|GetIsScanned (Class|SpmG5Character|GetItem (Variables|Default|GetInteracting%20Player))) (not (Variables|Default|GetIsBroken)))
            (CallFunction|SwapBox)
            (Variables|/Script/SpmG5.Item|SetbIsInStation (Variables|Default|GetScanningItem) true :!label _label_2)
            (CallFunction|StartSFX)
            (Transformation|AttachComponentToComponent (Variables|Default|GetScanningItem) (Variables|Default|GetBoxHolder) "None" "SnapToTarget" "SnapToTarget" "KeepRelative" true)
            (Rendering|SetVisibility (Variables|Default|GetSM_ScanDome) true false)
            (Rendering|SetVisibility (Variables|Default|GetScanDecal) true false)
            (bind _alpha (Timeline|ScanDomeScale PlayFromStart)
              (:Update
                (Transformation|SetRelativeScale3D (Variables|Default|GetSM_ScanDome) (Math|Vector|Lerp(Vector) "0.010000,0.010000,0.010000" "7.375000,7.375000,8.000000" _alpha)))
              (:Finished
                (Rendering|SetVisibility (Variables|Default|GetScanDecal) false false)
                (Rendering|SetVisibility (Variables|Default|GetSM_ScanDome) false false)
                (Niagara|SpawnSystematLocation "/Game/VFX/NS_UnpackingSmoke.NS_UnpackingSmoke" (Transformation|GetWorldLocation (Variables|Default|GetUnpackSmokeSpawn)))
                (Utilities|FlowControl|Delay (Variables|Default|GetDuration))
                (Variables|Default|SetisScanning false)
                (Utilities|IsValid (Variables|Default|GetScanningItem)
                  (:Is%20Valid
                    (Class|Item|SetIsInspected (Variables|Default|GetScanningItem) true)
                    (Class|Item|AddBonusPoints (Variables|Default|GetScanningItem) (Variables|/Script/SpmG5.Item|GetInspectedPoints (Variables|Default|GetScanningItem)))
                    (Variables|Default|SetVisibility true)
                    (if (CallFunction|GetIsBadItem (Variables|Default|GetScanningItem))
                      (bind _asdangerous_item (Utilities|Casting|CastToDangerousItem (Variables|Default|GetScanningItem))
                        (:then
                          _)
                        (:CastFailed
                          _))
                      ;[0.15 0.15 0.15 0.5] visa X dekal
                      (Rendering|Components|Decal|SetDecalMaterial (Actor|GetComponentbyClass (Variables|Default|GetScanningItem) "/Script/Engine.DecalComponent") "/Game/UI/Items/M_Decal_AddressXmark.M_Decal_AddressXmark")
                      (Rendering|SetVisibility (Actor|GetComponentbyClass (Variables|Default|GetScanningItem) "/Script/Engine.DecalComponent") (not (Utilities|IsValid _asdangerous_item)) false)
                      (bind _asbp_bomb (Utilities|Casting|CastToBP_Bomb (Variables|Default|GetScanningItem))
                        (:then
                          (Default|BecomeABomb _asbp_bomb)
                          (Class|DangerousItem|StartCountDownTimer _asbp_bomb))
                        (:CastFailed
                          _))
                      (Development|PrintString "This package is BAD" true true "(R=1.000000,G=0.084021,B=0.000000,A=1.000000)")
                      ;[0.15 0.15 0.15 0.5] Set SFX parameter - Ruben
                      (Class|FMODAudioComponent|SetParameter (Variables|Default|GetFMOD%20SFX) "Success" 0.0)
                      ;[0.15 0.15 0.15 0.5] Visar UI resultat
                      (Rendering|Material|SetMaterial (Variables|Default|GetUIPlane) 0 "/Game/UI/Popups/M_IconCross.M_IconCross")
                      (Rendering|SetVisibility (Variables|Default|GetParcelBad) true false)
                      (else
                        ;[0.15 0.15 0.15 0.5] Gå från att visa ? dekal till address dekal
                        (Class|Item|SetAddressDecal (Variables|Default|GetScanningItem))
                        ;[0.15 0.15 0.15 0.5] visa dekal
                        (Rendering|SetVisibility (Actor|GetComponentbyClass (Variables|Default|GetScanningItem) "/Script/Engine.DecalComponent") true false)
                        (Development|PrintString "This package is GOOD" true true "(R=0.143894,G=1.000000,B=0.206475,A=1.000000)")
                        (Class|FMODAudioComponent|SetParameter (Variables|Default|GetFMOD%20SFX) "Success" 1.0)
                        (Rendering|Material|SetMaterial (Variables|Default|GetUIPlane) 0 "/Game/UI/Popups/M_IconCheckmark.M_IconCheckmark")
                        (Rendering|SetVisibility (Variables|Default|GetParcelGood) true false)))
                    (Rendering|SetVisibility (Variables|Default|GetUIPlane) (Variables|Default|GetVisibility) false)
                    ;[0.15 0.15 0.15 0.5] Stop SFX and set it to null - Ruben
                    (Class|FMODAudioComponent|Stop (Variables|Default|GetFMOD%20SFX))
                    (Variables|Default|SetFMOD%20SFX 0)
                    (Variables|Default|SetTempHeldItem 0)))))
            (else
              (Rendering|Material|SetMaterial (Variables|Default|GetUIPlane) 0 "/Game/UI/Popups/M_IconScanFirst.M_IconScanFirst" :!label _label_3)
              (goto _label)))
          (else
            (CallFunction|PlayerPickup)))))
    (:Is%20Not%20Valid
      (if (not (Variables|Default|GetIsBroken))
        (if (Class|SpmG5Character|GetHasItem (Variables|Default|GetInteracting%20Player))
          (if (Class|Item|GetIsScanned (Class|SpmG5Character|GetItem (Variables|Default|GetInteracting%20Player)))
            (Variables|Default|SetisScanning true)
            (bind _returnvalue (Class|SpmG5Character|Drop (Variables|Default|GetInteracting%20Player)))
            (Variables|Default|SetScanningItem _returnvalue)
            (goto _label_2)
            (else
              (Development|PrintString "Scan your box first.")
              (goto _label_3)))
          (else
            (Development|PrintString "no box")
            (goto _label_3)))
        (else
          (CallFunction|Repair))))))

(event EventBreak
  ;[0.15 0.15 0.15 0.5] Machine breaking logic
  (Development|PrintString "THIS SHOULD BE BROKEN Hallå")
  (Variables|Default|SetIsBroken true)
  (Components|Activation|Activate (Variables|Default|GetBrokeSmoke) false))

(event EventCancelled
  ;[0.15 0.15 0.15 0.5] Machine breaking logic
  (Variables|/Script/SpmG5.SpmG5Character|SetIsRepairing (Variables|Default|GetInteracting%20Player) false)
  (Variables|/Script/SpmG5.SpmG5Character|SetRepairingActor (Variables|Default|GetInteracting%20Player) 0)
  (Utilities|Time|ClearandInvalidateTimerbyHandle (Variables|Default|GetRepairTimer))
  (Development|PrintString "FAHHHHHHHH"))

(event EventFinished
  ;[0.15 0.15 0.15 0.5] Machine breaking logic
  (Variables|Default|SetIsBroken false)
  (Variables|/Script/SpmG5.SpmG5Character|SetIsRepairing (Variables|Default|GetInteracting%20Player) false)
  (Variables|/Script/SpmG5.SpmG5Character|SetRepairingActor (Variables|Default|GetInteracting%20Player) 0)
  (Utilities|Time|ClearandInvalidateTimerbyHandle (Variables|Default|GetRepairTimer))
  (Development|PrintString "BANGERRRRRRRRRRRRR")
  (Components|Activation|Deactivate (Variables|Default|GetBrokeSmoke)))

(event EventRepair
  ;[0.15 0.15 0.15 0.5] Machine breaking logic
  (if (not (Utilities|Time|IsValidTimerHandle (Variables|Default|GetRepairTimer)))
    (Variables|/Script/SpmG5.SpmG5Character|SetIsRepairing (Variables|Default|GetInteracting%20Player) true)
    (Variables|/Script/SpmG5.SpmG5Character|SetRepairingActor (Variables|Default|GetInteracting%20Player) self)
    (Development|PrintString "bruh")
    (bind _returnvalue (Utilities|Time|SetTimerbyFunctionName 0 "FinishedCaller" (Variables|Default|GetRepairTime)))
    (Variables|Default|SetRepairTimer _returnvalue)))

(event EventBeginPlay
  (Utilities|FlowControl|Delay 0.2)
  (Transformation|SetWorldRotation (Variables|Default|GetUIPlane) (Math|Rotator|FindLookatRotation (Transformation|GetWorldLocation (Variables|Default|GetUIPlane)) (Variables|/Game/Blueprints/BP_GameManager.BP_GameManager_C|GetLevelCameraLocation (CallFunction|GetGameManager))) false false))

(fn ConstructionScript)

(fn StartSFX
  (if (Utilities|IsValid (Variables|Default|GetFMOD%20SFX))
    (Class|FMODAudioComponent|Stop (Variables|Default|GetFMOD%20SFX)))
  (bind _returnvalue (Class|FMODBlueprintStatics|PlayEventAttached "/Game/FMOD/Events/SFX/Stations/SFX_Scanner.SFX_Scanner" (Variables|Default|GetBoxHolder) "None" "0, 0, 0" "KeepRelativeOffset"))
  (Variables|Default|SetFMOD%20SFX _returnvalue))

(fn PlayerPickup
  (Transformation|DetachFromActor (Variables|Default|GetScanningItem) "KeepRelative" "KeepRelative" "KeepRelative")
  (Class|SpmG5Character|Pickup (Variables|Default|GetInteracting%20Player) (Variables|Default|GetScanningItem))
  (Variables|/Script/SpmG5.Item|SetbIsInStation (Variables|Default|GetScanningItem) false)
  (Variables|Default|SetScanningItem 0)
  (bind _output_get (Variables|Default|SetVisibility false))
  (Rendering|SetVisibility (Variables|Default|GetUIPlane) _output_get false)
  (Rendering|SetVisibility (Variables|Default|GetParcelGood) false false)
  (Rendering|SetVisibility (Variables|Default|GetParcelBad) false false))

(fn SwapBox
  (Variables|Default|SetTempHeldItem (Variables|/Script/SpmG5.SpmG5Character|GetHeldItem (Variables|Default|GetInteracting%20Player)))
  (Class|SpmG5Character|Drop (Variables|Default|GetInteracting%20Player))
  (Utilities|FlowControl|Sequence
    (:then_0
      (Niagara|SpawnSystematLocation "/Game/VFX/NS_SwitchPacketSmoke.NS_SwitchPacketSmoke" (Transformation|GetWorldLocation (Variables|Default|GetBoxHolder)) "0, 0, 0" "1.000000,1.000000,2.000000")
      (Niagara|SpawnSystematLocation "/Game/VFX/NS_SwitchPacketSmoke.NS_SwitchPacketSmoke" (Transformation|GetActorLocation (Variables|Default|GetTempHeldItem)) "0, 0, 0" "1.000000,1.000000,2.000000"))
    (:then_1
      (CallFunction|PlayerPickup)
      (Variables|Default|SetScanningItem (Variables|Default|GetTempHeldItem))
      (Variables|Default|SetisScanning true))))

(fn HandleThrow
  (params (Item :type Item%20Object%20Reference))
  (if (>= (.Z (Math|Vector|BreakVector (Transformation|GetActorLocation Item))) (+ (.Z (Math|Vector|BreakVector (Transformation|GetActorLocation))) 5e+01))
    (Utilities|IsValid (Variables|Default|GetScanningItem)
      (:Is%20Valid
        (return false))
      (:Is%20Not%20Valid
        (Development|PrintString "Should interact with item!!")
        (if (Class|Item|GetIsScanned Item)
          (Variables|Default|SetisScanning true)
          (Variables|Default|SetScanningItem Item)
          (return true))))
    (else
      (return false))))

(fn FinishedCaller
  (CallFunction|Finished))