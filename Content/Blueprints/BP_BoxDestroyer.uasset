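; BP_BoxDestroyer is an interactable disposal unit with a lid and dumpster smoke that destroys the item a player is carrying.
; On interact, it makes the player drop the held item, then shows a checkmark on UIPlane if the item is a DangerousItem, or a cross otherwise.
; The item disintegrates and the icon hides after a short delay.
; Smoke spawns at the lid on BeginPlay; the lid's hit event does nothing.
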(event OnComponentHit(LidMesh)
  (params (HitComponent :type Primitive%20Component%20Object%20Reference) (OtherActor :type Actor%20Object%20Reference) (OtherComp :type Primitive%20Component%20Object%20Reference) (NormalImpulse :type Vector :default "0, 0, 0") (Hit :type Hit%20Result%20Structure%20%28by%20ref%29)))

(event EventBeginPlay
  (Niagara|SpawnSystematLocation "/Game/VFX/NS_DumpsterSmoke.NS_DumpsterSmoke" (Transformation|GetWorldLocation (Variables|Default|GetLidMesh))))

(event EventOnInteract
  (params (InteractingPlayer :type Spm%20G5%20Character%20Object%20Reference))
  (if (Class|SpmG5Character|GetHasItem InteractingPlayer)
    (bind _returnvalue (Class|SpmG5Character|Drop InteractingPlayer))
    (Utilities|Casting|CastToDangerousItem _returnvalue
      (:then
        ;[0.15 0.15 0.15 0.5] Shows UI results
        (Rendering|Material|SetMaterial (Variables|Default|GetUIPlane) 0 "/Game/UI/M_IconCheckmark.M_IconCheckmark"))
      (:CastFailed
        (Rendering|Material|SetMaterial (Variables|Default|GetUIPlane) 0 "/Game/UI/M_IconCross.M_IconCross")))
    (Rendering|SetVisibility (Variables|Default|GetUIPlane) true false)
    (Class|Item|Disintegrate _returnvalue)
    (Utilities|FlowControl|Delay 1.5)
    (Rendering|SetVisibility (Variables|Default|GetUIPlane) false false)))

(fn ConstructionScript)